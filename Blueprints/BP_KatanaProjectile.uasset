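; Katana projectile that damages actors it overlaps, except the first-person character, and can fly back to the player.
; Entering or leaving a BP_WarpPoint overlap fires the warp dispatcher, and stopping the projectile pauses its trail.
; While ShouldReturnToPlayer is set, Tick steers it toward an offset from the player using both world offset and projectile velocity, blocking WorldDynamic.
; Once close to the player, it signals SwordReturned and destroys itself.
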(event `self.ReceiveActorBeginOverlap`
  (params (OtherActor :type "Actor Object Reference"))
  (cast `/Game/FirstPerson/Blueprints/BP_FirstPersonCharacter` OtherActor
    (:`CastFailed`
      (`GameplayStatics.ApplyDamage` OtherActor 100.0)
      (cast `/Game/FirstPerson/Blueprints/BP_WarpPoint` OtherActor)
      (`self.WarpDispatcher`))))

(event `self.ReceiveActorEndOverlap`
  (params (OtherActor :type "Actor Object Reference"))
  (cast `/Game/FirstPerson/Blueprints/BP_WarpPoint` OtherActor)
  (`self.WarpDispatcher`))

(event `self.ReceiveTick`
  (params (DeltaSeconds :type "Float (single-precision)"))
  (bind _returnvalue (`KismetMathLibrary.FindLookAtRotation` (`self.K2_GetActorLocation`) (+ (`self.K2_GetActorLocation` (`GameplayStatics.GetPlayerCharacter` 0)) (0.0 50.0 20.0))))
  (bind _returnvalue_2 (`KismetMathLibrary.GetForwardVector` _returnvalue))
  (if (`self.shouldReturnToPlayer`)
    (`self.K2_SetActorRotation` (`KismetMathLibrary.MakeRotator` (.roll _returnvalue) (.pitch _returnvalue) (+ (.yaw _returnvalue) -180.0)))
    (`self.K2_AddActorWorldOffset` (* _returnvalue_2 (`KismetMathLibrary.Conv_DoubleToVector` 100.0)))
    (`PrimitiveComponent.SetCollisionResponseToChannel` (`self.Box`) "ECC_WorldDynamic" "ECR_Block")
    (`PrimitiveComponent.SetCollisionResponseToChannel` (`self.katana`) "ECC_WorldDynamic" "ECR_Block")
    (set `MovementComponent.Velocity` (* _returnvalue_2 (`KismetMathLibrary.Conv_DoubleToVector` 6000.0)) (`self.ProjectileMovement`))
    (if (< (`KismetMathLibrary.Vector_Distance` (`self.K2_GetActorLocation`) (`self.K2_GetActorLocation` (`GameplayStatics.GetPlayerCharacter` 0))) 200.0)
      (`self.SwordReturned`)
      (`self.K2_DestroyActor`))))

(event `self.ProjectileMovement.OnProjectileStop`
  (params (ImpactResult :type "HitResult Structure (by ref)"))
  (`NiagaraComponent.SetPaused` (`self.Trail`) true))

(fn `UserConstructionScript`)