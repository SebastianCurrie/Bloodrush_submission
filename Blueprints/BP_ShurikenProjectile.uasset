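; Shuriken projectile that deals heavy damage to actors it overlaps, ignoring the first-person character.
; It destroys itself after damaging, unless the overlapped actor is a BP_Blood_Collision, which it passes without being destroyed.
; Tick spins it by adding a fixed pitch step each frame, independent of delta time, until a Hit event sets IsHit and stops the rotation.
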(event `self.ReceiveHit`
  (params (MyComp :type "PrimitiveComponent Object Reference") (Other :type "Actor Object Reference") (OtherComp :type "PrimitiveComponent Object Reference") (bSelfMoved :type Boolean) (HitLocation :type "Vector Structure") (HitNormal :type "Vector Structure") (NormalImpulse :type "Vector Structure") (Hit :type "HitResult Structure (by ref)"))
  (set `self.isHit` true))

(event `self.ReceiveActorBeginOverlap`
  (params (OtherActor :type "Actor Object Reference"))
  (cast `/Game/FirstPerson/Blueprints/BP_FirstPersonCharacter` OtherActor
    (:`CastFailed`
      (`GameplayStatics.ApplyDamage` OtherActor 100.0)
      (cast `/Game/FirstPerson/Effects/Blood/BP_Blood_Collision` OtherActor
        (:`CastFailed`
          (`self.K2_DestroyActor`))))))

(event `self.ReceiveTick`
  (params (DeltaSeconds :type "Float (single-precision)"))
  (if (not (`self.isHit`))
    (`self.K2_SetActorRotation` (`KismetMathLibrary.MakeRotator` (.roll (`self.K2_GetActorRotation`)) (+ (.pitch (`self.K2_GetActorRotation`)) 5.0) (.yaw (`self.K2_GetActorRotation`))))))

(fn `UserConstructionScript`)